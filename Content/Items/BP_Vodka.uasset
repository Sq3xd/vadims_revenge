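; BP_Vodka is a vodka item actor that shows a widget when the first-person character comes near.
; Its Sphere overlap begin and end events cast to BP_FirstPersonCharacter, then show or hide the Widget component.
; The same events enable or disable the actor's input for the player 0 controller, though the graph contains no input handlers or pickup logic.
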(event OnComponentBeginOverlap(Sphere)
  (params (OverlappedComponent :type Primitive%20Component%20Object%20Reference) (OtherActor :type Actor%20Object%20Reference) (OtherComp :type Primitive%20Component%20Object%20Reference) (OtherBodyIndex :type Integer) (bFromSweep :type Boolean) (SweepResult :type Hit%20Result%20Structure%20%28by%20ref%29))
  (Utilities|Casting|CastToBP_FirstPersonCharacter OtherActor)
  (Rendering|SetVisibility (Variables|Default|GetWidget) true false)
  (Input|EnableInput (Game|GetPlayerController (Variables|/Script/Engine.Pawn|GetPlayerState (Game|GetPlayerCharacter 0)))))

(event OnComponentEndOverlap(Sphere)
  (params (OverlappedComponent :type Primitive%20Component%20Object%20Reference) (OtherActor :type Actor%20Object%20Reference) (OtherComp :type Primitive%20Component%20Object%20Reference) (OtherBodyIndex :type Integer))
  (Utilities|Casting|CastToBP_FirstPersonCharacter OtherActor)
  (Rendering|SetVisibility (Variables|Default|GetWidget) false false)
  (Input|DisableInput (Game|GetPlayerController (Variables|/Script/Engine.Pawn|GetPlayerState (Game|GetPlayerCharacter 0)))))

(fn ConstructionScript)